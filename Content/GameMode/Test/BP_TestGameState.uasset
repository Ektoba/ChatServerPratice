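; Test game state for a turn-based baseball answer game, relaying chat messages, answer results and countdown updates to player controllers.
; A CurrentPlayer change resets the 15-second turn on the authority, ensures a looping one-second timer runs, and starts the turn on player controller 0.
; When time runs out, TurnOut submits a placeholder "/" answer for the current player and decrements their answers.
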(event Custom|MulticastTimeCountUpdate
  (params (Time :type Float%20%28double-precision%29))
  (Default|CallTimeCountUpdate Time))

(event Custom|BroadCastMessage
  (params (Message :type Text))
  (Default|CallAddChatMessage Message))

(event Custom|ClearTime
  (Utilities|Time|ClearTimerbyFunctionName 0 "TimeCountDown")
  (Utilities|Time|ClearandInvalidateTimerbyHandle (Variables|Default|GetTurnTimer)))

(event Custom|TurnOut
  (if (Utilities|Time|IsValidTimerHandle (Variables|Default|GetTurnTimer))
    (bind _asbp_test_controller (Utilities|Casting|CastToBP_TestController (Game|GetPlayerController 0)))
    (Default|BaseballLogic _asbp_test_controller (Variables|Default|GetCurrentPlayer) (Utilities|Text|FormatText "/"))
    (Default|DecrementAnswer (Variables|Default|GetCurrentPlayer))))

(event Custom|BroadCastAnswerState
  (params (ID :type Unique%20Net%20Id%20Repl%20Structure) (Answer :type Integer) (Result :type Baseball%20Result%20Structure))
  (bind _asbp_test_controller (Utilities|Casting|CastToBP_TestController (Game|GetPlayerController 0)))
  (Default|AnswerStateEvent _asbp_test_controller ID Answer Result))

(event Custom|BroadCastRemove
  (bind _asbp_test_controller (Utilities|Casting|CastToBP_TestController (Game|GetPlayerController 0)))
  (Utilities|IsValid (Variables|/Game/GameMode/Test/BP_TestController.BP_TestController_C|GetChatUI _asbp_test_controller)
    (:Is%20Valid
      (Default|RemoveItem (Variables|/Game/GameMode/Test/BP_TestController.BP_TestController_C|GetChatUI _asbp_test_controller)))))

(fn ConstructionScript)

(fn GetCurrentController
  (bind _asbp_test_controller (Utilities|Casting|CastToBP_TestController (Game|GetPlayerController 0)))
  (return _asbp_test_controller))

(fn OnRepCurrentPlayer
  (Networking|SwitchHasAuthority
    (:Authority
      (Utilities|FlowControl|Sequence
        (:then_0
          (Variables|Replication|SetServerStartTime (Utilities|Time|GetGameTimeinSeconds))
          (bind _output_get (Variables|Replication|SetTurnTime 15.0))
          (bind _output_get_2 (Variables|Replication|SetTurnTimeCount _output_get))
          (CallFunction|MulticastTimeCountUpdate _output_get_2))
        (:then_1
          (Utilities|FlowControl|Sequence
            (:then_0
              (if (Utilities|Time|IsValidTimerHandle (Variables|Default|GetTurnTimer))
                (Default|TurnStart (CallFunction|GetCurrentController))
                (else
                  (bind _returnvalue (Utilities|Time|SetTimerbyFunctionName 0 "TimeCountDown" 1.0 true))
                  (Variables|Default|SetTurnTimer _returnvalue)
                  (Default|TurnStart (CallFunction|GetCurrentController)))))))))))

(fn TimeCountDown
  (Networking|SwitchHasAuthority
    (:Authority
      (CallFunction|MulticastTimeCountUpdate (Variables|Replication|GetTurnTimeCount))
      (Math|Float|DecrementFloat (Variables|Replication|GetTurnTimeCount)
        (:%20%20
          (if (== (Variables|Replication|GetTurnTimeCount) -1.0)
            (CallFunction|TurnOut)))))))

(fn OnRepTurnTimeCount)