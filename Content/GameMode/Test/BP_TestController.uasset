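; Test player controller for a turn-based multiplayer baseball guessing game played through chat.
; After a short delay it creates the chat window, enables game-and-UI input and binds message and turn-timer events.
; BroadcastMessage posts chat through the GameState and forwards the current player's valid answers to the GameMode, which also handles turn switching.
; Number keys 1–4 are debug hooks that print or increment a PlayerState test integer through server/client-named events.
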(event Custom|PlayerStateClient
  (bind _asbp_test_player_state (Utilities|Casting|CastToBP_TestPlayerState (Variables|GetPlayerState)))
  (Development|PrintString (Utilities|String|Append "ClientTestInt : " (Utilities|String|ToString(Integer) (Variables|/Game/GameMode/Test/BP_TestPlayerState.BP_TestPlayerState_C|GetTestInt _asbp_test_player_state)))))

(event Custom|BroadcastMessage
  (params (Player :type BP%20Test%20Player%20State%20Object%20Reference) (Message :type Text))
  ;[0.15 0.15 0.15 0.5] 브로드캐스트
  (Utilities|FlowControl|Sequence
    (:then_0
      (CallFunction|ChatBroadCast Player Message))
    (:then_1
      (CallFunction|BaseballLogic Player Message))))

(event Custom|TimeCountUpdate_Event
  (params (Time :type Float%20%28double-precision%29))
  ;[0.15 0.15 0.15 0.5] UI_통신Event
  (Default|CallTimeCountUpdate Time))

(event Custom|CreateUI
  ;[0.15 0.15 0.15 0.5] Client의 위젯생성요청
  (Utilities|FlowControl|Sequence
    (:then_0
      (Utilities|IsValid (Variables|Default|GetChatUI)
        (:Is%20Not%20Valid
          (bind _returnvalue (UserInterface|CreateWidget "/Game/UI/WBP_ChatWindow.WBP_ChatWindow_C" self))
          (bind _output_get (Variables|Default|SetChatUI _returnvalue))
          (EventDispatchers|BindEventtoToServerMessage _output_get (EventDispatchers|CreateEvent :!event Custom|BroadcastMessage))
          (UserInterface|Viewport|AddtoViewport (Variables|Default|GetChatUI) 0))))
    (:then_1
      (Input|SetInputModeGameandUI self 0 "DoNotLock" false false)
      (Variables|Default|SetbShowMouseCursor true)
      (EventDispatchers|BindEventtoTimeCountUpdate (EventDispatchers|CreateEvent (Variables|Default|GetChatUI) :!event TimeCountUpdate))
      (bind _asbp_test_game_state (Utilities|Casting|CastToBP_TestGameState (Game|GetGameState)))
      (EventDispatchers|BindEventtoTimeCountUpdate _asbp_test_game_state (EventDispatchers|CreateEvent :!event Custom|TimeCountUpdate_Event)))))

(event Custom|PlayerStateServer
  (bind _asbp_test_player_state (Utilities|Casting|CastToBP_TestPlayerState (Variables|GetPlayerState)))
  (Development|PrintString (Utilities|String|Append "ServerTestInt : " (Utilities|String|ToString(Integer) (Variables|/Game/GameMode/Test/BP_TestPlayerState.BP_TestPlayerState_C|GetTestInt _asbp_test_player_state)))))

(event Custom|TurnOut
  ;[0.15 0.15 0.15 0.5] 턴을 바꾸는 것을 요청
  (Default|SwitchTrun (CallFunction|GetBPGameMode)))

(event Custom|TurnStart
  ;[0.15 0.15 0.15 0.5] 턴시작
  (Default|BroadCastMessage (CallFunction|GetBPGameState) (Utilities|Text|FormatText "<Server> : {0}님의 턴입니다." (Variables|/Game/GameMode/Test/BP_TestPlayerState.BP_TestPlayerState_C|GetSenderName (Default|CurrentUser (CallFunction|GetBPGameMode))))))

(event Custom|InputTestIntClient
  (bind _asbp_test_player_state (Utilities|Casting|CastToBP_TestPlayerState (Variables|GetPlayerState)))
  (Math|Integer|IncrementInt (Variables|/Game/GameMode/Test/BP_TestPlayerState.BP_TestPlayerState_C|GetTestInt _asbp_test_player_state)))

(event Custom|InputTestIntServer
  (bind _asbp_test_player_state (Utilities|Casting|CastToBP_TestPlayerState (Variables|GetPlayerState)))
  (Math|Integer|IncrementInt (Variables|/Game/GameMode/Test/BP_TestPlayerState.BP_TestPlayerState_C|GetTestInt _asbp_test_player_state)))

(event EventBeginPlay
  ;[0.15 0.15 0.15 0.5] UI배치
  (Utilities|FlowControl|Sequence
    (:then_0
      (Utilities|FlowControl|Delay 0.2)
      (if (Utilities|Enum|NotEqual(Enum) (Class|Actor|GetRemoteRole) "ROLE_None")
        (CallFunction|CreateUI)))))

(event Input|KeyboardEvents|1
  (params (Key :type Key%20Structure :default "None"))
  (:Pressed
    (CallFunction|PlayerStateServer)))

(event Input|KeyboardEvents|2
  (params (Key :type Key%20Structure :default "None"))
  (:Pressed
    (CallFunction|PlayerStateClient)))

(event Input|KeyboardEvents|3
  (params (Key :type Key%20Structure :default "None"))
  (:Pressed
    (CallFunction|InputTestIntServer)))

(event Input|KeyboardEvents|4
  (params (Key :type Key%20Structure :default "None"))
  (:Pressed
    (CallFunction|InputTestIntClient)))

(fn ConstructionScript)

(fn BaseballLogic
  (params (PlayerState :type BP%20Test%20Player%20State%20Object%20Reference) (Answer :type Text%20%28by%20ref%29))
  (bind _returnvalue (CallFunction|GetBPGameMode))
  (if (== (CallFunction|GetCurrentTurnPlayer) PlayerState)
    (Utilities|FlowControl|Sequence
      (:then_0
        (bind _returnvalue_2 (Class|ChatGameMode|AnswerCheck _returnvalue Answer))
        (if _returnvalue_2
          (Default|ReceiveAnswer _returnvalue PlayerState Answer))))))

(fn ChatBroadCast
  (params (PlayerState :type BP%20Test%20Player%20State%20Object%20Reference) (Message :type Text))
  (Default|BroadCastMessage (.AsBP%20Test%20Game%20State (Utilities|Casting|CastToBP_TestGameState (Game|GetGameState))) (Utilities|Text|FormatText "{0} : {1}" (Variables|/Game/GameMode/Test/BP_TestPlayerState.BP_TestPlayerState_C|GetSenderName PlayerState) Message)))

(fn GetBPGameState
  (return (.AsBP%20Test%20Game%20State (Utilities|Casting|CastToBP_TestGameState (Game|GetGameState)))))

(fn GetCurrentTurnPlayer
  (return (Variables|/Game/GameMode/Test/BP_TestGameState.BP_TestGameState_C|GetCurrentPlayer (CallFunction|GetBPGameState))))

(fn GetBPGameMode
  (bind _asbp_test_game_mode (Utilities|Casting|CastToBP_TestGameMode (Game|GetGameMode))
    (:then
      (return _asbp_test_game_mode))
    (:CastFailed
      (Development|PrintText "GameController->Casting GameMode실패"))))

(fn GetBPPlayerState
  (bind _asbp_test_player_state (Utilities|Casting|CastToBP_TestPlayerState (Variables|GetPlayerState)))
  (return _asbp_test_player_state))