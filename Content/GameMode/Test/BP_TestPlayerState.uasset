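; Test PlayerState for a networked, turn-based answer game, tracking each player's remaining answer count and win, loss or draw outcome.
; BeginPlay sets an init flag whose RepNotify, on authority, has the game mode assign an ID to players other than player 0.
; Decrementing the count ends the controller's turn and flags a loss at zero, reporting it to the game mode.
; RepNotifies refresh the count UI and show Korean result messages.
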(event Custom|SetLoginID
  (params (PlayerState :type BP%20Test%20Player%20State%20Object%20Reference))
  (Default|AssignID (Utilities|GetServerGameMode) PlayerState))

(event Custom|SetDraw
  (Variables|Default|SetbIsDraw true)
  (CallFunction|ShowResult true "무승부 입니다."))

(event Custom|SetAnswer
  (params (Answer :type Integer))
  (bind _output_get (Variables|Default|SetAnswerCount Answer))
  (CallFunction|SendUI _output_get)
  (Default|PlayerLoseIncrement (Utilities|GetServerGameMode)))

(event Custom|ShowResult
  (params (Open :type Boolean) (Message :type Text))
  (Default|CallShowResultUI Open Message))

(event Custom|SendUI
  (params (Answer :type Integer))
  (Default|CallUpdateUI Answer))

(event Custom|DecrementAnswer
  (bind _result (Math|Integer|DecrementInt (Variables|Default|GetAnswerCount))
    (:%20%20
      (Default|CallUpdateUI _result)
      (Default|TurnOut (Utilities|GetLocalPlayerController))
      (if (== (Variables|Default|GetAnswerCount) 0)
        (CallFunction|SetLose true)))))

(event Custom|SetLose
  (params (Lose :type Boolean))
  (Variables|Default|SetbIsLose Lose)
  (Default|PlayerLoseIncrement (Utilities|GetServerGameMode)))

(event EventBeginPlay
  (Variables|Default|SetbIsInitialize true))

(fn ConstructionScript)

(fn OnRepSenderName)

(fn OnRepBIsInitialize
  ;[0.15 0.15 0.15 0.5] 서버에서 실행되어야 클라이언트로 복제가 된다.
  (Networking|SwitchHasAuthority
    (:Authority
      (if (!= (Game|GetPlayerController 0) (Game|GetPlayerController))
        (CallFunction|SetLoginID self)))))

(fn OnRepAnswerCount
  (Default|CallUpdateUI (Variables|Default|GetAnswerCount)))

(fn OnRepBIsLose
  (if (Variables|Default|GetbIsLose)
    (Default|CallShowResultUI true "패배하셨습니다.")
    (elif (not (== (Variables|Default|GetAnswerCount) 3))
      (Default|CallShowResultUI true "승리하셨습니다."))))

(fn OnRepTestInt
  (Development|PrintString (Utilities|String|Append "OnRepTestInt : " (Utilities|String|ToString(Integer) (Variables|Default|GetTestInt)))))

(fn OnRepBIsDraw
  (Default|CallShowResultUI true "무승부 입니다."))